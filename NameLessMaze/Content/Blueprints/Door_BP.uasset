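; Door Blueprint that swings open and shut, optionally automatically when the player character enters or leaves its trigger volume.
; Trigger begin and end overlaps check the AutoOpen or AutoClose flag and the IsClosed state, then share a call to ToggleDoor.
; ToggleDoor flips IsClosed and plays or reverses a timeline that lerps the door's relative yaw between closed and a quarter turn open.
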(event `self.Trigger.OnComponentBeginOverlap`
  (params (OverlappedComponent :type "PrimitiveComponent Object Reference") (OtherActor :type "Actor Object Reference") (OtherComp :type "PrimitiveComponent Object Reference") (OtherBodyIndex :type Integer) (bFromSweep :type Boolean) (SweepResult :type "HitResult Structure (by ref)"))
  ;[1 1 1] Proximity open/close
  (if (and (`self.AutoOpen`) (== OtherActor (`GameplayStatics.GetPlayerCharacter` 0)) (`self.IsClosed`))
    (`self.ToggleDoor` :!label _label)))

(event `ToggleDoor`
  ;[1 1 1] Toggle Door
  (if (`self.IsClosed`)
    (set `self.IsClosed` false)
    (bind (_direction _alpha) (`Timeline|OpenDoor_TL` :!label _label_2)
      (:`Update`
        (`SceneComponent.K2_SetRelativeRotation` (`self.Door`) (`KismetMathLibrary.MakeRotator` 0.0 0.0 (`KismetMathLibrary.Lerp` 0.0 90.0 _alpha)) false false)))
    (else
      (set `self.IsClosed` true)
      (goto _label_2 :!via `Reverse`))))

(event `self.Trigger.OnComponentEndOverlap`
  (params (OverlappedComponent :type "PrimitiveComponent Object Reference") (OtherActor :type "Actor Object Reference") (OtherComp :type "PrimitiveComponent Object Reference") (OtherBodyIndex :type Integer))
  ;[1 1 1] Proximity open/close
  (if (and (== (`GameplayStatics.GetPlayerCharacter` 0) OtherActor) (`self.AutoClose`) (not (`self.IsClosed`)))
    (goto _label)))

(fn `UserConstructionScript`)