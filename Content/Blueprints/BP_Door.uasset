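; BP_Door is a door actor that slides between two positions in response to a TurnSwitch event.
; The Active flag selects one of two hard-coded world locations, offset along Y, and SetActorLocation moves the door there instantly without sweep or interpolation.
; The absolute coordinates tie the Blueprint to one placement in a level; its other events and construction script add no logic.
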(event `/Game/Blueprints/TurnSwitch_BP.TurnSwitch`
  (params (`Active?` :type Boolean))
  (if `Active?`
    (`self.K2_SetActorLocation` (18250.0 4280.0 1170.0))
    (else
      (`self.K2_SetActorLocation` (18250.0 4520.0 1170.0)))))

(fn `UserConstructionScript`
  (`parent.UserConstructionScript`))