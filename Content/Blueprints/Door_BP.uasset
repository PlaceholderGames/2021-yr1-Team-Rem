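; A swinging door that can open and close automatically on player proximity and be unlocked with a keypad code.
; A trigger overlap shrinks the player's capsule near the door and restores it on exit, then calls open or close, gated by auto flags and lock state.
; A timeline rotates the door's yaw, reversing to close, with sounds.
; CheckCode compares KeyPad_UI entries, unlocking and opening on a match and clearing the entry either way.
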(event `self.Trigger.OnComponentBeginOverlap`
  (params (OverlappedComponent :type "PrimitiveComponent Object Reference") (OtherActor :type "Actor Object Reference") (OtherComp :type "PrimitiveComponent Object Reference") (OtherBodyIndex :type Integer) (bFromSweep :type Boolean) (SweepResult :type "HitResult Structure (by ref)"))
  ;[1 1 1] Proximity open/close
  (`|ExecutionSequence`
    (:`then_0`
      (`self.SetPlayerCapsuleRadius` OtherActor 30.0))
    (:`then_1`
      (`self.OpenDoorOnPlayerEntry` OtherActor))))

(event `ToggleDoor`
  ;[1 1 1] Door Control
  (if (`self.IsClosed`)
    (set `self.IsClosed` false :!label _label)
    (bind (_direction _alpha) (`Timeline|OpenDoor_TL` :!label _label_2)
      (:`Update`
        (`SceneComponent.K2_SetRelativeRotation` (`self.Door`) (`KismetMathLibrary.MakeRotator` 0.0 0.0 (`KismetMathLibrary.Lerp` 0.0 90.0 _alpha)) false false)))
    (else
      (set `self.IsClosed` true :!label _label_3)
      (goto _label_2 :!via `Reverse`))))

(event `OpenDoor`
  ;[1 1 1] Door Control
  (if (`self.IsClosed`)
    (`GameplayStatics.PlaySound2D` "/Game/Sounds/OpenDoor.OpenDoor" 1.0 1.0 0.0 null null)
    (`|ExecutionSequence`
      (:`then_0`
        (goto _label))
      (:`then_1`
        (`KismetSystemLibrary.PrintString` "Opening the door!")))))

(event `self.Trigger.OnComponentEndOverlap`
  (params (OverlappedComponent :type "PrimitiveComponent Object Reference") (OtherActor :type "Actor Object Reference") (OtherComp :type "PrimitiveComponent Object Reference") (OtherBodyIndex :type Integer))
  ;[1 1 1] Proximity open/close
  (`|ExecutionSequence`
    (:`then_0`
      (`self.SetPlayerCapsuleRadius` OtherActor))
    (:`then_1`
      (`self.CloseDoorOnPlayerExit` OtherActor))))

(event `CloseDoor`
  ;[1 1 1] Door Control
  (if (not (`self.IsClosed`))
    (`GameplayStatics.PlaySound2D` "/Game/Sounds/CloseDoor.CloseDoor" 1.0 1.0 0.0 null null)
    (`|ExecutionSequence`
      (:`then_0`
        (goto _label_3))
      (:`then_1`
        (`KismetSystemLibrary.PrintString` "Closing the door!")))))

(event `self.ReceiveBeginPlay`
  (bind _askey_pad_ui (cast `/Game/Blueprints/UI/KeyPad_UI` (`WidgetComponent.GetUserWidgetObject` (`self.Widget`))))
  (bind _output_get (set `self.KeyPad_UI` _askey_pad_ui))
  (add `/Game/Blueprints/UI/KeyPad_UI.CodeEntered` _output_get (`|CreateDelegate` :!event `CheckCode`)))

(fn `CheckCode`
  (params (CodeEntered :type String) (KeyPad_UI :type "/Game/Blueprints/UI/KeyPad_UI Object Reference"))
  (if (`KismetStringLibrary.EqualEqual_StrStr` CodeEntered (`self.CorrectCode`))
    (set `self.Locked` false)
    (`self.OpenDoor`)
    (set `/Game/Blueprints/UI/KeyPad_UI.CurrentCode` "" (`self.KeyPad_UI`))
    (else
      (set `/Game/Blueprints/UI/KeyPad_UI.CurrentCode` "" (`self.KeyPad_UI`)))))

(fn `UserConstructionScript`)